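; BP_Player is the player character for the Android VR POC app, steering its view from device motion.
; BeginPlay creates the Player_HUD widget and adds it to the viewport.
; Each Tick feeds the motion rotation rate, scaled by TURN, LOOK and delta time, into controller yaw and pitch.
; A sword draw/sheathe montage toggle based on SwordEquipped exists but is not connected to any input or event.
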(event `self.ReceiveBeginPlay`
  (bind _returnvalue (`|CreateWidget` "/Game/AndroidVrPocApp/Player/UI/Player_HUD.Player_HUD_C"))
  (`UserWidget.AddToViewport` _returnvalue 0))

(event `self.ReceiveTick`
  (params (DeltaSeconds :type "Float (single-precision)"))
  (bind (_tilt _rotationrate) (`PlayerController.GetInputMotionState` (`GameplayStatics.GetPlayerController` 0)))
  (`|ExecutionSequence`
    (:`then_0`
      (`self.AddControllerYawInput` (* (.x _rotationrate) (`self.tURN`) (`GameplayStatics.GetWorldDeltaSeconds`))))
    (:`then_1`
      (`self.AddControllerPitchInput` (* (.y _rotationrate) (`self.lOOK`) (`GameplayStatics.GetWorldDeltaSeconds`))))))

(fn `UserConstructionScript`)